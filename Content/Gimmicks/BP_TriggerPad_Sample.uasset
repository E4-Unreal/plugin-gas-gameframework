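; BP_TriggerPad_Sample is a sample trigger pad gimmick that shows its active state by swapping the material on its display mesh.
; It overrides TryActivate and TryDeactivate, calling the parent first and applying ActivateMaterial or DeactivateMaterial to slot 0 only when that call succeeds.
; Both overrides return the parent's result, and the event graph and construction script add no logic.
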(fn `TryActivate`
  (params (InCauser :type "Actor Object Reference") (InInstigator :type "Actor Object Reference"))
  (returns (ReturnValue :type Boolean))
  (bind _returnvalue (`parent.TryActivate` InCauser InInstigator))
  (if _returnvalue
    (`PrimitiveComponent.SetMaterial` (`self.DisplayMesh`) 0 (`self.ActivateMaterial`)))
  (return _returnvalue))

(fn `TryDeactivate`
  (params (InCauser :type "Actor Object Reference") (InInstigator :type "Actor Object Reference"))
  (returns (ReturnValue :type Boolean))
  (bind _returnvalue (`parent.TryDeactivate` InCauser InInstigator))
  (if _returnvalue
    (`PrimitiveComponent.SetMaterial` (`self.DisplayMesh`) 0 (`self.DeactivateMaterial`)))
  (return _returnvalue))

(fn `UserConstructionScript`)